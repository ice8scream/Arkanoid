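; BlocksGenerator_BP is an actor that spawns a grid of Block_BP actors when play begins.
; Nested loops over X and Y counts place each block at a Padding-based offset from the generator's location, on a flat XY plane.
; XScale and YScale size each block, and YScale also stretches the Y spacing, while X spacing ignores XScale.
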(event `self.ReceiveBeginPlay`
  (for _index (range (`self.X`))
    (for _index_2 (range (`self.Y`))
      (`|SpawnActorFromClass` "/Game/Block_BP.Block_BP_C" (`KismetMathLibrary.MakeTransform` (+ (`self.K2_GetActorLocation`) (`KismetMathLibrary.MakeVector` (`KismetMathLibrary.Conv_IntToDouble` (* _index (`self.Padding`))) (* (`KismetMathLibrary.Conv_IntToDouble` (* _index_2 (`self.Padding`))) (`self.YScale`)))) (struct) (`KismetMathLibrary.MakeVector` (`self.XScale`) (`self.YScale`) 1.0)) "Undefined" "OverrideRootScale" null null))))

(fn `UserConstructionScript`)