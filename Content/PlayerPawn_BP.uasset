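; PlayerPawn_BP is the player paddle in a ball game, moving sideways on input and managing the ball's lives.
; It spawns a Ball_BP at BallSpawnPoint, listens for its death and respawns it after a delay until MaxDeadCount is reached, then plays a sound.
; On a hit, it briefly waits, then blends its last move direction into the ball's direction.
; PlayPowerUp grants an extra life, ignoring its Num input.
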(event `self.ReceiveBeginPlay`
  (`self.SpawnBall`))

(event `InputAxis|MoveHorisontal`
  (params (AxisValue :type "Float (single-precision)"))
  (bind _returnvalue (* AxisValue (`self.Speed`) (`GameplayStatics.GetWorldDeltaSeconds`)))
  (`self.K2_AddActorWorldOffset` (`KismetMathLibrary.MakeVector` 0.0 _returnvalue))
  (set `self.LastMoveDirection` (`KismetMathLibrary.MakeVector` 0.0 _returnvalue)))

(event `SpawnBall`
  (bind _returnvalue (`|SpawnActorFromClass` "/Game/Ball_BP.Ball_BP_C" (`KismetMathLibrary.MakeTransform` (`SceneComponent.K2_GetComponentLocation` (`self.BallSpawnPoint`)) (struct :`Yaw` 45.0) (0.5 0.5 0.5)) "AdjustIfPossibleButAlwaysSpawn" "OverrideRootScale" null null))
  (add `/Game/Ball_BP.OnDead` _returnvalue (delegate `Ball Dead`)))

(event `Ball Dead`
  (`/Engine/EditorBlueprintResources/StandardMacros.IncrementInt` (`self.DeadCount`)
    (:`  `
      (`KismetSystemLibrary.PrintString` "ball dead")
      (`KismetSystemLibrary.Delay` 1.0)
      (if (< (`self.DeadCount`) (`self.MaxDeadCount`))
        (`self.SpawnBall`)
        (else
          (`GameplayStatics.PlaySound2D` "/Engine/EditorSounds/Notifications/CompileFailed_Cue.CompileFailed_Cue" 1.0 1.0 0.0 null null))))))

(event `self.ReceiveHit`
  (params (MyComp :type "PrimitiveComponent Object Reference") (Other :type "Actor Object Reference") (OtherComp :type "PrimitiveComponent Object Reference") (bSelfMoved :type Boolean) (HitLocation :type "Vector Structure") (HitNormal :type "Vector Structure") (NormalImpulse :type "Vector Structure") (Hit :type "HitResult Structure (by ref)"))
  (bind _asball_bp (cast `/Game/Ball_BP` Other))
  (`KismetSystemLibrary.Delay` 0.05)
  (set `/Game/Ball_BP.Ball Direction` (`KismetMathLibrary.Normal` (+ (`/Game/Ball_BP.Ball Direction` _asball_bp) (`KismetMathLibrary.Normal` (`self.LastMoveDirection`)))) _asball_bp))

(event `self.ReceiveActorBeginOverlap`
  (params (OtherActor :type "Actor Object Reference")))

(event `Play Power Up`
  (params (num :type Integer))
  (`/Engine/EditorBlueprintResources/StandardMacros.IncrementInt` (`self.MaxDeadCount`)))

(fn `UserConstructionScript`)