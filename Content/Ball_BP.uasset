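; Ball actor that travels in a straight line, bounces off blocking surfaces and dies in a kill volume.
; Tick moves it along BallDirection with a swept offset, then reflects the direction about the hit normal and plays a sound on impact.
; Overlapping a KillZVolume calls OnDead, destroys the ball and plays an eject sound.
; Speed-decrease logic clamped to MinSpeed exists but is unconnected.
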(event `self.ReceiveBeginPlay`
  (set `self.Ball Direction` (`self.GetActorForwardVector`)))

(event `self.ReceiveTick`
  (params (DeltaSeconds :type "Float (single-precision)"))
  (bind _sweephitresult (`self.K2_AddActorWorldOffset` (* (`self.Ball Direction`) (* DeltaSeconds (`self.BallSpeed`))) true))
  (bind (_bblockinghit _binitialoverlap _time _distance _location _impactpoint _normal _impactnormal _physmat _hitactor _hitcomponent _hitbonename _hititem _faceindex _tracestart _traceend) (`GameplayStatics.BreakHitResult` _sweephitresult))
  (if _bblockinghit
    (set `self.Ball Direction` (`KismetMathLibrary.GetReflectionVector` (`KismetMathLibrary.GetDirectionUnitVector` _tracestart _traceend) _normal))
    (`GameplayStatics.PlaySound2D` "/Engine/VREditor/Sounds/UI/Camera_Shutter.Camera_Shutter" 1.0 1.0 0.0 null null)))

(event `self.ReceiveActorBeginOverlap`
  (params (OtherActor :type "Actor Object Reference"))
  (cast `KillZVolume` OtherActor)
  (`self.OnDead`)
  (`self.K2_DestroyActor`)
  (`GameplayStatics.PlaySound2D` "/Engine/EditorSounds/GamePreview/EjectFromPlayer_Cue.EjectFromPlayer_Cue" 1.0 1.0 0.0 null null))

(event `self.ReceiveHit`
  (params (MyComp :type "PrimitiveComponent Object Reference") (Other :type "Actor Object Reference") (OtherComp :type "PrimitiveComponent Object Reference") (bSelfMoved :type Boolean) (HitLocation :type "Vector Structure") (HitNormal :type "Vector Structure") (NormalImpulse :type "Vector Structure") (Hit :type "HitResult Structure (by ref)")))

(fn `UserConstructionScript`)