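; A power-up pickup actor that drifts along negative world X with a text label for its randomly chosen type.
; BeginPlay picks one of four types and shows its label: S, L, M or +1.
; Tick moves it with a swept offset scaled by speed and delta time.
; Overlap with a kill volume destroys it; the player pawn first gets PlayPowerUp, always passed 0 rather than the rolled type.
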(event `self.ReceiveBeginPlay`
  (set `self.PowerupNum` (`KismetMathLibrary.RandomIntegerInRange` 0 3))
  (switch `int` (`self.PowerupNum`)
    (:`0`
      (set `self.PoverUpName` "S"))
    (:`1`
      (set `self.PoverUpName` "L"))
    (:`2`
      (set `self.PoverUpName` "M"))
    (:`3`
      (set `self.PoverUpName` "+1")))
  (`TextRenderComponent.K2_SetText` (`self.PowerUpName`) (`KismetTextLibrary.Conv_StringToText` (`self.PoverUpName`))))

(event `self.ReceiveTick`
  (params (DeltaSeconds :type "Float (single-precision)"))
  (`self.K2_AddActorWorldOffset` (`KismetMathLibrary.MakeVector` (* DeltaSeconds (`self.PowerUpSpeed`) -1.0)) true))

(event `self.ReceiveActorBeginOverlap`
  (params (OtherActor :type "Actor Object Reference"))
  (cast `KillZVolume` OtherActor
    (:`then`
      _)
    (:`CastFailed`
      (bind _asplayer_pawn_bp (cast `/Game/PlayerPawn_BP` OtherActor))
      (`/Game/PlayerPawn_BP.Play Power Up` _asplayer_pawn_bp 0)))
  (`self.K2_DestroyActor`))

(fn `UserConstructionScript`)