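; Block_BP is a breakable block that takes two hits to destroy and can spawn an actor when it breaks.
; The first Hit event swaps the Cube's material to a green one and sets the WasHit flag.
; A later hit rolls a one-in-three chance to spawn an actor, whose class is unspecified here, at the block's location, then destroys the block.
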(event `self.ReceiveHit`
  (params (MyComp :type "PrimitiveComponent Object Reference") (Other :type "Actor Object Reference") (OtherComp :type "PrimitiveComponent Object Reference") (bSelfMoved :type Boolean) (HitLocation :type "Vector Structure") (HitNormal :type "Vector Structure") (NormalImpulse :type "Vector Structure") (Hit :type "HitResult Structure (by ref)"))
  (if (`self.bWasHit`)
    (if (> (`KismetMathLibrary.RandomInteger` 9) 5)
      (`|SpawnActorFromClass` "/Game/PowerUp_BP.PowerUp_BP_C" (`KismetMathLibrary.MakeTransform` (`self.K2_GetActorLocation`) (struct) (1.0 1.0 1.0)) "Undefined" "OverrideRootScale" null null))
    (`self.K2_DestroyActor`)
    (else
      (`PrimitiveComponent.SetMaterial` (`self.Cube`) 0 "/Engine/EngineDebugMaterials/VertexColorViewMode_GreenOnly.VertexColorViewMode_GreenOnly")
      (set `self.bWasHit` true))))

(fn `UserConstructionScript`)